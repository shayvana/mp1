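; BP_EnemySpawner spawns BP_Enemy actors, creating the first at a fixed location on BeginPlay.
; SpawnEnemy stores each new enemy as NewestEnemy and gives it a reference back to the spawner.
; SpawnEnemyAtSpawnPoint chains placement by spawning the next enemy at the newest one's SpawnPoint component, though nothing in this Blueprint calls it.
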(event `self.ReceiveBeginPlay`
  (`self.SpawnEnemy` (3000.0 0.0 0.0)))

(fn `SpawnEnemy`
  (params (SpawnLocation :type "Vector Structure"))
  (bind _returnvalue (`|SpawnActorFromClass` "/Game/InfiniteMatrix/Blueprints/BP_Enemy.BP_Enemy_C" (`KismetMathLibrary.MakeTransform` SpawnLocation) "Undefined" "OverrideRootScale" null null))
  (bind _output_get (set `self.NewestEnemy` _returnvalue))
  (set `/Game/InfiniteMatrix/Blueprints/BP_Enemy.EnemySpawner` self _output_get))

(fn `SpawnEnemyAtSpawnPoint`
  (`self.SpawnEnemy` (`SceneComponent.K2_GetComponentLocation` (`/Game/InfiniteMatrix/Blueprints/BP_Enemy.SpawnPoint` (`self.NewestEnemy`)))))

(fn `UserConstructionScript`)