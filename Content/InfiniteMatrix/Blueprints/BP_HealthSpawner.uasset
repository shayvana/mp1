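; BP_HealthSpawner is an actor that spawns chained BP_HealthPack pickups.
; On BeginPlay it spawns the first pack at a fixed location, stores it as the newest pack and gives it a back-reference to the spawner.
; SpawnHealthPackAtSpawnPoint spawns the next pack at the newest pack's SpawnPoint component, extending the chain; nothing in this Blueprint calls it.
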(event `self.ReceiveBeginPlay`
  (`self.SpawnHealthPack` (3000.0 0.0 0.0)))

(fn `SpawnHealthPack`
  (params (SpawnLocation :type "Vector Structure"))
  (bind _returnvalue (`|SpawnActorFromClass` "/Game/InfiniteMatrix/Blueprints/BP_HealthPack.BP_HealthPack_C" (`KismetMathLibrary.MakeTransform` SpawnLocation) "Undefined" "OverrideRootScale" null null))
  (bind _output_get (set `self.NewestHealthPack` _returnvalue))
  (set `/Game/InfiniteMatrix/Blueprints/BP_HealthPack.HealthSpawner` self _output_get))

(fn `SpawnHealthPackAtSpawnPoint`
  (`self.SpawnHealthPack` (`SceneComponent.K2_GetComponentLocation` (`/Game/InfiniteMatrix/Blueprints/BP_HealthPack.SpawnPoint` (`self.NewestHealthPack`)))))

(fn `UserConstructionScript`)